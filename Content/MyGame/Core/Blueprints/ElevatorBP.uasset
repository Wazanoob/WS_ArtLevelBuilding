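; Elevator actor that the player calls with the Interact input while standing in its trigger, making a round trip between start and end positions.
; Trigger overlap by the ThirdPersonCharacter toggles this actor's input and an on-screen prompt widget.
; A Timeline lerps the Elevator component's relative location.
; On finish, a FlipFlop alternates between a delayed reverse and re-arming the origin flag, which blocks re-triggering mid-trip.
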(event OnComponentBeginOverlap(trigger)
  (params (OverlappedComponent :type Primitive%20Component%20Object%20Reference) (OtherActor :type Actor%20Object%20Reference) (OtherComp :type Primitive%20Component%20Object%20Reference) (OtherBodyIndex :type Integer) (bFromSweep :type Boolean) (SweepResult :type Hit%20Result%20Structure%20%28by%20ref%29))
  (Utilities|Casting|CastToThirdPersonCharacter OtherActor)
  (Input|EnableInput (Game|GetPlayerController 0))
  ;[1 1 1] Add and remove widget from screen
  (bind _returnvalue (UserInterface|CreateWidget "/Game/MyGame/Widget/InputEWidget.InputEWidget_C"))
  (UserInterface|Viewport|AddtoViewport _returnvalue 0))

(event OnComponentEndOverlap(trigger)
  (params (OverlappedComponent :type Primitive%20Component%20Object%20Reference) (OtherActor :type Actor%20Object%20Reference) (OtherComp :type Primitive%20Component%20Object%20Reference) (OtherBodyIndex :type Integer))
  (Utilities|Casting|CastToThirdPersonCharacter OtherActor)
  (Input|DisableInput (Game|GetPlayerController 0))
  ;[1 1 1] Add and remove widget from screen
  (Widget|RemovefromParent (stale OnComponentBeginOverlap(trigger) _returnvalue)))

(event Input|ActionEvents|InputActionInteract
  (params (Key :type Key%20Structure))
  (:Pressed
    (if (Variables|Default|GetisOnOriginPos)
      (Utilities|FlowControl|Sequence
        (:then_0
          (Variables|Default|SetisOnOriginPos false)
          (bind _elevatormovement (Timeline|Timeline_0 Play)
            (:Update
              (Transformation|SetRelativeLocation (Variables|Default|GetElevator) (Math|Vector|Lerp(Vector) (Variables|Default|GetStartPos) (Variables|Default|GetEndPos) _elevatormovement) false false))
            (:Finished
              (Utilities|FlowControl|FlipFlop
                (:A
                  (Utilities|FlowControl|Delay 3.0)
                  (Timeline|Timeline_0 Reverse))
                (:B
                  (Variables|Default|SetisOnOriginPos true))))))
        (:then_1
          (Development|PrintString "GoingUp"))))))

(fn ConstructionScript)