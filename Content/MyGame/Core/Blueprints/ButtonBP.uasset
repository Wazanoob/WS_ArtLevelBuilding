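; Interactable button actor that lets the player open a ButtonDoorBP door.
; Its Trigger overlap enables input and shows an InputEWidget prompt while the ThirdPersonCharacter is inside, undoing both on exit.
; Pressing Interact finds the door with GetActorOfClass rather than a set reference, calls OpenDoor with the player character, and switches the player's view target to the door.
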(event OnComponentBeginOverlap(trigger)
  (params (OverlappedComponent :type Primitive%20Component%20Object%20Reference) (OtherActor :type Actor%20Object%20Reference) (OtherComp :type Primitive%20Component%20Object%20Reference) (OtherBodyIndex :type Integer) (bFromSweep :type Boolean) (SweepResult :type Hit%20Result%20Structure%20%28by%20ref%29))
  (Utilities|Casting|CastToThirdPersonCharacter OtherActor)
  (Input|EnableInput (Game|GetPlayerController 0))
  ;[1 1 1] Add and remove widget from screen
  (bind _returnvalue (UserInterface|CreateWidget "/Game/MyGame/Widget/InputEWidget.InputEWidget_C"))
  (UserInterface|Viewport|AddtoViewport _returnvalue 0))

(event OnComponentEndOverlap(trigger)
  (params (OverlappedComponent :type Primitive%20Component%20Object%20Reference) (OtherActor :type Actor%20Object%20Reference) (OtherComp :type Primitive%20Component%20Object%20Reference) (OtherBodyIndex :type Integer))
  (Utilities|Casting|CastToThirdPersonCharacter OtherActor)
  (Input|DisableInput (Game|GetPlayerController 0))
  ;[1 1 1] Add and remove widget from screen
  (Widget|RemovefromParent (stale OnComponentBeginOverlap(trigger) _returnvalue)))

(event Input|ActionEvents|InputActionInteract
  (params (Key :type Key%20Structure))
  (:Pressed
    (bind _returnvalue (Actor|GetActorOfClass "/Game/MyGame/Core/Blueprints/ButtonDoorBP.ButtonDoorBP_C"))
    (Default|OpenDoor _returnvalue (Game|GetPlayerCharacter 0))
    (Game|Player|SetViewTargetwithBlend (Game|GetPlayerController 0) _returnvalue 0.0 "VTBlend_Linear" 0.0 false)))

(fn ConstructionScript)